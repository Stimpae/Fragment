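; BP_Platforms is a configurable tilemap platform that is solid to pawns only while the player is inside its trigger box.
; The construction script applies the chosen tile map and sets the box's extent and relative location from variables.
; When BP_PlayerCharacter enters the box, the tile map's Pawn response switches to Block, and on exit it switches to Overlap, allowing pass-through platform behavior.
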(event `self.Box.OnComponentBeginOverlap`
  (params (OverlappedComponent :type "PrimitiveComponent Object Reference") (OtherActor :type "Actor Object Reference") (OtherComp :type "PrimitiveComponent Object Reference") (OtherBodyIndex :type Integer) (bFromSweep :type Boolean) (SweepResult :type "HitResult Structure (by ref)"))
  (cast `/Game/Player/BP_PlayerCharacter` OtherActor)
  (`PrimitiveComponent.SetCollisionResponseToChannel` (`self.PaperTileMap`) "ECC_Pawn" "ECR_Block"))

(event `self.Box.OnComponentEndOverlap`
  (params (OverlappedComponent :type "PrimitiveComponent Object Reference") (OtherActor :type "Actor Object Reference") (OtherComp :type "PrimitiveComponent Object Reference") (OtherBodyIndex :type Integer))
  (cast `/Game/Player/BP_PlayerCharacter` OtherActor)
  (`PrimitiveComponent.SetCollisionResponseToChannel` (`self.PaperTileMap`) "ECC_Pawn" "ECR_Overlap"))

(fn `UserConstructionScript`
  (`PaperTileMapComponent.SetTileMap` (`self.PaperTileMap`) (`self.NewTileMap`))
  (`BoxComponent.SetBoxExtent` (`self.Box`) (`self.BoxExtent`) true)
  (`SceneComponent.K2_SetRelativeLocation` (`self.Box`) (`self.BoxLocation`) false false))