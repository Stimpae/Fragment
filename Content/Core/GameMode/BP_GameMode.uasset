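; BP_GameMode is the game mode that coordinates respawning after the player dies and relays fog control.
; BeginPlay caches references to the player character and the first BP_Fog actor in the level.
; Respawn respawns the character, resets the fog, then respawns every BP_CoinSpawner, with the coin step running only if the fog reference is valid.
; SetFogStopped forwards its flag to the fog, and GetGameWidgets is an empty stub.
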(event `self.ReceiveBeginPlay`
  ;[1 1 1] Create reference to player character
  (`/Engine/EditorBlueprintResources/StandardMacros.IsValid` (`self.CharacterReference`)
    (:`Is Valid`
      _)
    (:`Is Not Valid`
      (bind _asbp_player_character (cast `/Game/Player/BP_PlayerCharacter` (`GameplayStatics.GetPlayerCharacter` 0)))
      (set `self.CharacterReference` _asbp_player_character)))
  ;[1 1 1] Create reference to fog
  (bind _outactors (`GameplayStatics.GetAllActorsOfClass` "/Game/Core/Mechanics/Fog/BP_Fog.BP_Fog_C"))
  (set `self.FogReference` (`|GetArrayItem` _outactors)))

(event `/Game/Core/Interfaces/BPI_GameInterface.Respawn`
  (bind _characterreference (`self.CharacterReference`))
  (bind _fogreference (`self.FogReference`))
  ;[1 1 1] Respawns the character and fog after character death
  (`/Engine/EditorBlueprintResources/StandardMacros.IsValid` _characterreference
    (:`Is Valid`
      (`/Game/Player/BP_PlayerCharacter.Respawn` _characterreference)
      (`/Engine/EditorBlueprintResources/StandardMacros.IsValid` _fogreference
        (:`Is Valid`
          (`/Game/Core/Mechanics/Fog/BP_Fog.ResetFog` _fogreference)
          ;[1 1 1] Respawn all coins
          (bind _outactors (`GameplayStatics.GetAllActorsOfClass` "/Game/Core/Mechanics/Coins/BP_CoinSpawner.BP_CoinSpawner_C"))
          (for _array_element _outactors
            (`/Game/Core/Mechanics/Coins/BP_CoinSpawner.Respawn` _array_element)))))))

(event `/Game/Core/Interfaces/BPI_GameInterface.SetFogStopped`
  (params (`Stopped?` :type Boolean))
  (`/Game/Core/Mechanics/Fog/BP_Fog.SetFogStopped` (`self.FogReference`) `Stopped?`))

(fn `GetGameWidgets`
  (returns (MainMenu :type "/Game/Widgets/WBP_MainMenu Object Reference") (InGame :type "/Game/Widgets/WBP_InGame Object Reference") (LevelSelect :type "/Game/Widgets/WBP_LevelSelect Object Reference") (GameOver :type "/Game/Widgets/WBP_GameOver Object Reference"))
  (return null null null null))

(fn `UserConstructionScript`)