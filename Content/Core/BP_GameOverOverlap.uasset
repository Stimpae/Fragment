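; BP_GameOverOverlap is a trigger box that ends the game when BP_PlayerCharacter enters it, with its extent set from OverlapBoxSize in the construction script.
; On overlap it pauses the game after a short delay and, in parallel, plays the in-game widget's fade animation in reverse.
; After the fade delay, the game instance displays a message widget.
; A sound node, noted for possible falling sounds, is left unconnected.
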(event `self.Overlap.OnComponentBeginOverlap`
  (params (OverlappedComponent :type "PrimitiveComponent Object Reference") (OtherActor :type "Actor Object Reference") (OtherComp :type "PrimitiveComponent Object Reference") (OtherBodyIndex :type Integer) (bFromSweep :type Boolean) (SweepResult :type "HitResult Structure (by ref)"))
  (bind _asbp_player_character (cast `/Game/Player/BP_PlayerCharacter` OtherActor))
  (bind _output_get (set `self.CharacterReference` _asbp_player_character))
  (`/Engine/EditorBlueprintResources/StandardMacros.IsValid` _output_get
    (:`Is Valid`
      (`|ExecutionSequence`
        (:`then_0`
          (`KismetSystemLibrary.Delay` 0.4)
          (`GameplayStatics.SetGamePaused` true))
        (:`then_1`
          (bind (_mainmenu _ingame) (message `/Game/Core/Interfaces/BPI_GameInterface.GetGameWidgets` (`GameplayStatics.GetGameInstance`)))
          (bind _finishtime (`/Game/Widgets/WBP_InGame.FadeAnimation` _ingame "Reverse" 0.8))
          (`KismetSystemLibrary.Delay` _finishtime)
          (message `/Game/Core/Interfaces/BPI_GameInterface.DisplayWidgets` (`GameplayStatics.GetGameInstance`) "NewEnumerator4"))))))

(fn `UserConstructionScript`
  (`BoxComponent.SetBoxExtent` (`self.Overlap`) (`self.OverlapBoxSize`) true))