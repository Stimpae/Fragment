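; BP_LevelManager tracks the currently selected level and modifier indices for a menu of level and modifier buttons.
; SetCurrentButtons passes the manager to every button in both arrays through SetMenuManager.
; Two setter events store the chosen index and print it to the screen for debugging.
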(event `/Game/Core/Interfaces/BPI_MenuInterface.SetLevelIndex`
  (params (Index :type Integer))
  (bind _output_get (set `self.CurrentLevelIndex` Index))
  (`KismetSystemLibrary.PrintString` null (`KismetStringLibrary.Conv_IntToString` _output_get)))

(event `/Game/Core/Interfaces/BPI_MenuInterface.SetModifierIndex`
  (params (Index :type Integer))
  (bind _output_get (set `self.CurrentModifierIndex` Index))
  (`KismetSystemLibrary.PrintString` null (`KismetStringLibrary.Conv_IntToString` _output_get)))

(fn `SetCurrentButtons`
  (params (InLevelButtons :type "Array of /Game/Widgets/WBP_LevelButton Object Reference") (InModifierButtons :type "Array of /Game/Widgets/WBP_ModifierLevels Object Reference"))
  (for _array_element InLevelButtons
    (`/Game/Widgets/WBP_LevelButton.SetMenuManager` _array_element self))
  (for _array_element_2 InModifierButtons
    (`/Game/Widgets/WBP_ModifierLevels.SetMenuManager` _array_element_2 self)))