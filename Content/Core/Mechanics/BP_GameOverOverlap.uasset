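; Trigger box actor that ends the game when BP_PlayerCharacter overlaps it.
; On overlap it stores the character, pauses the game after a short delay, and plays the in-game widget's fade animation in reverse.
; After a delay based on that fade, it asks the game instance to display the game-over widget.
; The construction script sizes the box from OverlapBoxSize; a sound node is left unconnected.
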(event `self.Overlap.OnComponentBeginOverlap`
  (params (OverlappedComponent :type "PrimitiveComponent Object Reference") (OtherActor :type "Actor Object Reference") (OtherComp :type "PrimitiveComponent Object Reference") (OtherBodyIndex :type Integer) (bFromSweep :type Boolean) (SweepResult :type "HitResult Structure (by ref)"))
  ;[1 1 1] Checks overlap is the character, if true creates a ref
  (bind _asbp_player_character (cast `/Game/Player/BP_PlayerCharacter` OtherActor))
  (bind _output_get (set `self.CharacterReference` _asbp_player_character))
  (`/Engine/EditorBlueprintResources/StandardMacros.IsValid` _output_get
    (:`Is Valid`
      (`|ExecutionSequence`
        (:`then_0`
          ;[1 1 1] Set game paused to avoid other things happening to char
          (`KismetSystemLibrary.Delay` 0.4)
          (`GameplayStatics.SetGamePaused` true))
        (:`then_1`
          ;[1 1 1] Fade out in game widget
          (bind (_mainmenu _ingame) (message `/Game/Core/Interfaces/BPI_GameInterface.GetGameWidgets` (`GameplayStatics.GetGameInstance`)))
          (bind _finishtime (`/Game/Widgets/WBP_InGame.FadeAnimation` _ingame "Reverse" 0.8))
          (`KismetSystemLibrary.Delay` _finishtime)
          ;[1 1 1] Display game over
          (message `/Game/Core/Interfaces/BPI_GameInterface.DisplayWidgets` (`GameplayStatics.GetGameInstance`) "NewEnumerator4"))))))

(fn `UserConstructionScript`
  (`BoxComponent.SetBoxExtent` (`self.Overlap`) (`self.OverlapBoxSize`) true))