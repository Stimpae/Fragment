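; BP_CoinSpawner is an actor that spawns a straight row of BP_Coins along the world X axis from its own location.
; A loop offsets each coin by index times SpaceBetweenCoins from the truncated starting X, keeping the spawner's Y and Z, with NumberOfCoins bounding the loop.
; BeginPlay and the Respawn event share this logic, and neither removes previously spawned coins.
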(event `Respawn`
  (bind _returnvalue_x (`KismetMathLibrary.BreakVector` (`self.K2_GetActorLocation`)))
  (bind (_returnvalue_x_2 _returnvalue_y _returnvalue_z) (`KismetMathLibrary.BreakVector` (`self.K2_GetActorLocation`)))
  (set `self.StartingXLocation` _returnvalue_x :!label _label)
  (for _index (range (+ (`self.NumberOfCoins`) 1))
    (`|SpawnActorFromClass` "/Game/Core/Mechanics/Coins/BP_Coins.BP_Coins_C" (`KismetMathLibrary.MakeTransform` (`KismetMathLibrary.MakeVector` (`KismetMathLibrary.Conv_IntToDouble` (+ (* _index (`self.SpaceBetweenCoins`)) (`KismetMathLibrary.FTrunc` (`self.StartingXLocation`)))) _returnvalue_y _returnvalue_z)) "Undefined" "OverrideRootScale" null null)))

(event `self.ReceiveBeginPlay`
  (goto _label))

(fn `UserConstructionScript`)