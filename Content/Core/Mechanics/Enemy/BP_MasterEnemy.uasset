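; Master 2D side-scroller enemy that patrols along X, reversing on capsule hits, with flipbook animation driven by velocity.
; Player overlap with the outer sphere runs a looping, randomly timed Fire that spawns projectiles both ways, paused inside the inner sphere or on exit.
; DeathCollision launches the player and destroys the enemy, while KnockbackCollision flings the player and zeroes their MovementScale.
; The construction script applies sphere radii and walk speed from variables.
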(event `self.Sphere.OnComponentBeginOverlap`
  (params (OverlappedComponent :type "PrimitiveComponent Object Reference") (OtherActor :type "Actor Object Reference") (OtherComp :type "PrimitiveComponent Object Reference") (OtherBodyIndex :type Integer) (bFromSweep :type Boolean) (SweepResult :type "HitResult Structure (by ref)"))
  ;[1 1 1] Comment
  (bind _asbp_player_character (cast `/Game/Player/BP_PlayerCharacter` OtherActor))
  (`/Engine/EditorBlueprintResources/StandardMacros.IsValid` _asbp_player_character
    (:`Is Valid`
      (if (`KismetSystemLibrary.K2_IsValidTimerHandle` (`self.FireTimerHandle`))
        (`KismetSystemLibrary.K2_UnPauseTimerHandle` (`self.FireTimerHandle`))
        (else
          (bind _returnvalue (`KismetSystemLibrary.K2_SetTimer` null "Fire" (`KismetMathLibrary.RandomFloatInRange` 1.4 2.0) true))
          (set `self.FireTimerHandle` _returnvalue))))))

(event `self.ReceiveTick`
  (params (DeltaSeconds :type "Float (single-precision)"))
  ;[1 1 1] Tick
  (`self.CheckMovement`)
  (`self.Direction`))

(event `self.ReceiveBeginPlay`
  ;[1 1 1] Begin Play
  (`self.UpdateAnimations` "NewEnumerator0"))

(event `self.DeathCollision.OnComponentBeginOverlap`
  (params (OverlappedComponent :type "PrimitiveComponent Object Reference") (OtherActor :type "Actor Object Reference") (OtherComp :type "PrimitiveComponent Object Reference") (OtherBodyIndex :type Integer) (bFromSweep :type Boolean) (SweepResult :type "HitResult Structure (by ref)"))
  ;[1 1 1] when the player character overlaps with the box above the enemy, launch the character and destroy enemy
  (bind _asbp_player_character (cast `/Game/Player/BP_PlayerCharacter` OtherActor))
  (`/Engine/EditorBlueprintResources/StandardMacros.IsValid` _asbp_player_character
    (:`Is Valid`
      (`self.LaunchCharacter` _asbp_player_character (50.0 0.0 50.0) true true)
      (`self.K2_DestroyActor`))))

(event `self.Sphere.OnComponentEndOverlap`
  (params (OverlappedComponent :type "PrimitiveComponent Object Reference") (OtherActor :type "Actor Object Reference") (OtherComp :type "PrimitiveComponent Object Reference") (OtherBodyIndex :type Integer))
  ;[1 1 1] Comment
  (bind _asbp_player_character (cast `/Game/Player/BP_PlayerCharacter` OtherActor))
  (`/Engine/EditorBlueprintResources/StandardMacros.IsValid` _asbp_player_character
    (:`Is Valid`
      (`KismetSystemLibrary.K2_PauseTimerHandle` (`self.FireTimerHandle`)))))

(event `self.CapsuleComponent.OnComponentHit`
  (params (HitComponent :type "PrimitiveComponent Object Reference") (OtherActor :type "Actor Object Reference") (OtherComp :type "PrimitiveComponent Object Reference") (NormalImpulse :type "Vector Structure") (Hit :type "HitResult Structure (by ref)"))
  ;[1 1 1] Toggles when the enemy comes into contact with a collision (used to move back and forth
  (castclass `/Game/Core/Mechanics/Enemy/BP_Projectile` (`GameplayStatics.GetObjectClass` (`.HitActor` (`GameplayStatics.BreakHitResult` Hit)))
    (:`CastFailed`
      (set `self.isMovingRight` (not (`self.isMovingRight`))))))

(event `self.KnockbackCollision.OnComponentBeginOverlap`
  (params (OverlappedComponent :type "PrimitiveComponent Object Reference") (OtherActor :type "Actor Object Reference") (OtherComp :type "PrimitiveComponent Object Reference") (OtherBodyIndex :type Integer) (bFromSweep :type Boolean) (SweepResult :type "HitResult Structure (by ref)"))
  (bind _asbp_player_character (cast `/Game/Player/BP_PlayerCharacter` OtherActor))
  (`/Engine/EditorBlueprintResources/StandardMacros.IsValid` _asbp_player_character
    (:`Is Valid`
      (set `/Game/Player/BP_PlayerCharacter.MovementScale` 0.0 _asbp_player_character)
      (`self.LaunchCharacter` _asbp_player_character (-400.0 0.0 400.0) true true))))

(event `self.InnerSphere.OnComponentBeginOverlap`
  (params (OverlappedComponent :type "PrimitiveComponent Object Reference") (OtherActor :type "Actor Object Reference") (OtherComp :type "PrimitiveComponent Object Reference") (OtherBodyIndex :type Integer) (bFromSweep :type Boolean) (SweepResult :type "HitResult Structure (by ref)"))
  (bind _asbp_player_character (cast `/Game/Player/BP_PlayerCharacter` OtherActor))
  (`/Engine/EditorBlueprintResources/StandardMacros.IsValid` _asbp_player_character
    (:`Is Valid`
      (`KismetSystemLibrary.K2_PauseTimerHandle` (`self.FireTimerHandle`)))))

(event `self.InnerSphere.OnComponentEndOverlap`
  (params (OverlappedComponent :type "PrimitiveComponent Object Reference") (OtherActor :type "Actor Object Reference") (OtherComp :type "PrimitiveComponent Object Reference") (OtherBodyIndex :type Integer))
  (bind _asbp_player_character (cast `/Game/Player/BP_PlayerCharacter` OtherActor))
  (`/Engine/EditorBlueprintResources/StandardMacros.IsValid` _asbp_player_character
    (:`Is Valid`
      (`KismetSystemLibrary.K2_UnPauseTimerHandle` (`self.FireTimerHandle`)))))

(fn `CheckMovement`
  (bind _returnvalue (`|EnumInequality` (`self.CurrentAnimationState`) "NewEnumerator2"))
  (bind _velocity_x (`KismetMathLibrary.BreakVector` (`MovementComponent.Velocity` (`self.GetMovementComponent`))))
  (bind _velocity_x_2 (`KismetMathLibrary.BreakVector` (`MovementComponent.Velocity` (`self.GetMovementComponent`))))
  (if (or (> _velocity_x 0.0) (< _velocity_x_2 0.0))
    (if _returnvalue
      (`self.UpdateAnimations` "NewEnumerator1"))
    (elif _returnvalue
      (`self.UpdateAnimations` "NewEnumerator0"))))

(fn `Direction`
  (`SceneComponent.K2_SetRelativeRotation` (`self.Sprite`) (`KismetMathLibrary.MakeRotator` 0.0 0.0 (`KismetMathLibrary.SelectFloat` 0.0 180.0 (`self.isMovingRight`))) false false)
  (`self.AddMovementInput` (`KismetMathLibrary.SelectVector` (1.0 0.0 0.0) (-1.0 0.0 0.0) (`self.isMovingRight`))))

(fn `Fire`
  (bind (_returnvalue_x _returnvalue_y _returnvalue_z) (`KismetMathLibrary.BreakVector` (`SceneComponent.K2_GetComponentLocation` (`self.Sprite`))))
  (bind (_returnvalue_x_2 _returnvalue_y_2 _returnvalue_z_2) (`KismetMathLibrary.BreakVector` (`SceneComponent.K2_GetComponentLocation` (`self.Sprite`))))
  (`KismetSystemLibrary.PrintString` "Hello" true true (struct :`G` 0.66 :`B` 1.0 :`A` 1.0) 0.1)
  (`|ExecutionSequence`
    (:`then_0`
      (`|SpawnActorFromClass` "/Game/Core/Mechanics/Enemy/BP_Projectile.BP_Projectile_C" (`KismetMathLibrary.MakeTransform` (`KismetMathLibrary.MakeVector` (+ _returnvalue_x_2 -50.0) _returnvalue_y_2 _returnvalue_z_2) (struct :`Yaw` 180.0)) "AdjustIfPossibleButAlwaysSpawn" "OverrideRootScale" null null))
    (:`then_1`
      (`|SpawnActorFromClass` "/Game/Core/Mechanics/Enemy/BP_Projectile.BP_Projectile_C" (`KismetMathLibrary.MakeTransform` (`KismetMathLibrary.MakeVector` (+ _returnvalue_x 50.0) _returnvalue_y _returnvalue_z)) "AdjustIfPossibleButAlwaysSpawn" "OverrideRootScale" null null))))

(fn `UpdateAnimations`
  (params (AnimState :type "/Game/Core/Enums/E_AnimationStates Enum" :default "NewEnumerator0"))
  (switch `/Game/Core/Enums/E_AnimationStates` AnimState
    (:`NewEnumerator0`
      (set `self.CurrentAnimationState` "NewEnumerator0"))
    (:`NewEnumerator1`
      (set `self.CurrentAnimationState` "NewEnumerator1"))
    (:`NewEnumerator2`
      (set `self.CurrentAnimationState` "NewEnumerator2"))
    (:`NewEnumerator3`
      (set `self.CurrentAnimationState` "NewEnumerator2")))
  (`PaperFlipbookComponent.SetFlipbook` (`self.Sprite`) (select `/Game/Core/Enums/E_AnimationStates` (`self.CurrentAnimationState`) :`NewEnumerator0` (`self.IdleFlipbook`) :`NewEnumerator1` (`self.RunFlipbook`) :`NewEnumerator2` (`self.JumpingFlipbook`) :`NewEnumerator3` (`self.LandingFlipbook`))))

(fn `UserConstructionScript`
  (`SphereComponent.SetSphereRadius` (`self.Sphere`) (`self.SphereRadius`) true)
  (`SphereComponent.SetSphereRadius` (`self.InnerSphere`) (`self.InnerSphereRadius`) true)
  (set `CharacterMovementComponent.MaxWalkSpeed` (`self.MovementSpeed`) (`self.CharacterMovement`)))