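; BP_Fog is an advancing fog hazard that triggers game over when its collision box overlaps the player character.
; Tick moves it along X by MovementSpeed per frame, without delta-time scaling, unless FogStopped is set.
; Overlap fades out the in-game widget and shows game over, but sets FogStopped false despite its comment saying it stops.
; ResetFog returns it to its BeginPlay location and resumes movement after a short delay.
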(event `ResetFog`
  ;[1 1 1] Set location to default start
  (`self.K2_SetActorLocation` (`self.StartingLocation`))
  ;[1 1 1] allow time for game over widget to fade
  (`KismetSystemLibrary.Delay` 0.5)
  ;[1 1 1] Restart fog movement
  (set `self.FogStopped` false))

(event `/Game/Core/Interfaces/BPI_GameInterface.SetFogStopped`
  (params (`Stopped?` :type Boolean))
  ;[1 1 1] Set fogged stopped
  (set `self.FogStopped` `Stopped?`))

(event `self.ReceiveBeginPlay`
  ;[1 1 1] Set default starting location
  (set `self.StartingLocation` (`self.K2_GetActorLocation`)))

(event `self.ReceiveTick`
  (params (DeltaSeconds :type "Float (single-precision)"))
  (bind (_returnvalue_x _returnvalue_y _returnvalue_z) (`KismetMathLibrary.BreakVector` (`self.K2_GetActorLocation`)))
  ;[1 1 1] EVENT TICK - changes the actors location on the x axis depending on the movement speed float set
  (if (not (`self.FogStopped`))
    (`self.K2_SetActorLocation` (`KismetMathLibrary.MakeVector` (+ _returnvalue_x (`self.MovementSpeed`)) _returnvalue_y _returnvalue_z))))

(event `self.CollisionBox.OnComponentBeginOverlap`
  (params (OverlappedComponent :type "PrimitiveComponent Object Reference") (OtherActor :type "Actor Object Reference") (OtherComp :type "PrimitiveComponent Object Reference") (OtherBodyIndex :type Integer) (bFromSweep :type Boolean) (SweepResult :type "HitResult Structure (by ref)"))
  ;[1 1 1] Creates reference to playerbp on overlap
  (bind _asbp_player_character (cast `/Game/Player/BP_PlayerCharacter` OtherActor))
  (`/Engine/EditorBlueprintResources/StandardMacros.IsValid` _asbp_player_character
    (:`Is Valid`
      ;[1 1 1] Fades out in game widget
      (bind (_mainmenu _ingame) (message `/Game/Core/Interfaces/BPI_GameInterface.GetGameWidgets` (`GameplayStatics.GetGameInstance`)))
      (bind _finishtime (`/Game/Widgets/WBP_InGame.FadeAnimation` _ingame "Reverse" 0.8))
      (`KismetSystemLibrary.Delay` _finishtime)
      ;[1 1 1] displays game over and stops fog from moving any furthur
      (message `/Game/Core/Interfaces/BPI_GameInterface.DisplayWidgets` (`GameplayStatics.GetGameInstance`) "NewEnumerator4")
      (set `self.FogStopped` false))))

(fn `GetGameWidgets`
  (returns (MainMenu :type "/Game/Widgets/WBP_MainMenu Object Reference") (InGame :type "/Game/Widgets/WBP_InGame Object Reference") (LevelSelect :type "/Game/Widgets/WBP_LevelSelect Object Reference") (GameOver :type "/Game/Widgets/WBP_GameOver Object Reference"))
  (return null null null null))

(fn `UserConstructionScript`
  (`SceneComponent.SetWorldScale3D` (`self.FogSprite`) (`self.FogSize`)))