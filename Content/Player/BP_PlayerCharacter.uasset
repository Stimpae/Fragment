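; Flipbook-animated player character that moves along world X at MovementScale, independent of axis value, with configurable jumps triggered by input or events.
; Tick switches idle/running flipbooks from velocity and runs a debug landing-prediction trace; landing briefly adjusts braking friction.
; Timed debuffs lower walk speed until a timer restores it.
; BeginPlay registers the character with the game instance; Respawn unpauses, teleports to PlayerStart and fades the in-game widget.
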(event `Respawn`
  ;[1 1 1] Respawn
  (`GameplayStatics.SetGamePaused` false)
  (bind _outactors (`GameplayStatics.GetAllActorsOfClass` "/Script/Engine.PlayerStart"))
  (bind _output (`|GetArrayItem` _outactors))
  (`self.K2_SetActorLocationAndRotation` self (`self.K2_GetActorLocation` _output) (`self.K2_GetActorRotation` _output) false true)
  (`self.UpdateAnimations` "NewEnumerator0")
  (bind (_mainmenu _ingame) (message `/Game/Core/Interfaces/BPI_GameInterface.GetGameWidgets` (`GameplayStatics.GetGameInstance`)))
  (`/Game/Widgets/WBP_InGame.FadeAnimation` _ingame "Forward" 1.0)
  (set `self.MovementScale` 1.0))

(event `self.OnLanded`
  (params (Hit :type "HitResult Structure (by ref)"))
  (bind _charactermovement (`self.CharacterMovement`))
  (bind _velocity_x (`KismetMathLibrary.BreakVector` (`MovementComponent.Velocity` (`self.GetMovementComponent`))))
  ;[1 1 1] On Landed
  (if (> _velocity_x 0.0)
    (`self.UpdateAnimations` "NewEnumerator1")
    (set `CharacterMovementComponent.BrakingFrictionFactor` 0.5 _charactermovement)
    (else
      (`self.UpdateAnimations` "NewEnumerator0")
      (set `CharacterMovementComponent.BrakingFrictionFactor` 3.0 _charactermovement)))
  (`KismetSystemLibrary.Delay` 0.2)
  (set `CharacterMovementComponent.BrakingFrictionFactor` 0.0 (`self.CharacterMovement`))
  (`self.UpdateAnimations` "NewEnumerator1")
  (set `self.MovementScale` 1.0))

(event `self.ReceiveTick`
  (params (DeltaSeconds :type "Float (single-precision)"))
  (bind (_returnvalue_x _returnvalue_y _returnvalue_z) (`KismetMathLibrary.BreakVector` (`self.K2_GetActorLocation`)))
  (bind _capsulecomponent (`self.CapsuleComponent`))
  (bind (_velocity_x _velocity_y _velocity_z) (`KismetMathLibrary.BreakVector` (`MovementComponent.Velocity` (`self.GetMovementComponent`))))
  (bind _returnvalue (`KismetMathLibrary.MakeVector` _returnvalue_x _returnvalue_y (- _returnvalue_z (`CapsuleComponent.GetScaledCapsuleHalfHeight_WithoutHemisphere` _capsulecomponent))))
  ;[1 1 1] Tick
  (`self.CheckMovement`)
  (if (`NavMovementComponent.IsFalling` (`self.CharacterMovement`))
    (`KismetSystemLibrary.SphereTraceSingle` :`Start` _returnvalue :`End` (+ _returnvalue (* (`KismetMathLibrary.Normal` (`KismetMathLibrary.MakeVector` _velocity_x _velocity_y (`KismetMathLibrary.FClamp` _velocity_z -4000.0 -200.0))) (`KismetMathLibrary.MapRangeClamped` _velocity_z 0.0 -4000.0 50.0 2000.0))) :`Radius` (`CapsuleComponent.GetScaledCapsuleRadius` _capsulecomponent) :`TraceChannel` "TraceTypeQuery1" :`DrawTime` 0.0)))

(event `self.ReceiveBeginPlay`
  ;[1 1 1] Begin Play
  (`self.UpdateAnimations` "NewEnumerator0")
  (message `/Game/Core/Interfaces/BPI_GameInterface.CreateCharacterReference` (`GameplayStatics.GetGameInstance`) self))

(event `InputAction|Jump`
  (params (Key :type "Key Structure"))
  ;[1 1 1] Handle Jump
  (:`Pressed`
    (if (`self.CanJump`) :!label _label
      (`self.UpdateAnimations` "NewEnumerator2")
      (`self.Jump`)))
  (:`Released`
    (`self.StopJumping` :!label _label_2)))

(event `JumpEvent`
  ;[1 1 1] Handle Jump
  (goto _label))

(event `ReleasedEvent`
  ;[1 1 1] Handle Jump
  (goto _label_2))

(event `InputAxis|MoveRight`
  (params (AxisValue :type "Float (single-precision)"))
  ;[1 0 0] Debug // Movement //
  (`self.AddMovementInput` (1.0 0.0 0.0) (`self.MovementScale`)))

(fn `CheckMovement`
  (bind _returnvalue (`|EnumInequality` (`self.CurrentAnimationState`) "NewEnumerator2"))
  (bind _velocity_x (`KismetMathLibrary.BreakVector` (`MovementComponent.Velocity` (`self.GetMovementComponent`))))
  (bind _velocity_x_2 (`KismetMathLibrary.BreakVector` (`MovementComponent.Velocity` (`self.GetMovementComponent`))))
  (if (or (> _velocity_x 0.0) (< _velocity_x_2 0.0))
    (if _returnvalue
      (`self.UpdateAnimations` "NewEnumerator1"))
    (elif _returnvalue
      (`self.UpdateAnimations` "NewEnumerator0"))))

(fn `DebuffPlayerSpeed`
  (params (Amount :type "Float (double-precision)") (DebuffTime :type "Float (double-precision)"))
  (locals (LAmount :type "Float (double-precision)") (LDebuffTime :type "Float (double-precision)"))
  (set `local.LAmount` Amount)
  (set `local.LDebuffTime` DebuffTime)
  (set `CharacterMovementComponent.MaxWalkSpeed` (- (`self.DefaultMovementSpeed`) (`local.LAmount`)) (`self.CharacterMovement`))
  (if (`KismetSystemLibrary.K2_IsValidTimerHandle` (`self.DebuffTimerHandle`))
    (`KismetSystemLibrary.K2_UnPauseTimerHandle` (`self.DebuffTimerHandle`)))
  (bind _returnvalue (`KismetSystemLibrary.K2_SetTimer` null "SetDefaultPlayerSpeed" (`local.LDebuffTime`)))
  (set `self.DebuffTimerHandle` _returnvalue))

(fn `SetDefaultPlayerSpeed`
  (set `CharacterMovementComponent.MaxWalkSpeed` (`self.DefaultMovementSpeed`) (`self.CharacterMovement`))
  (`KismetSystemLibrary.K2_PauseTimerHandle` (`self.DebuffTimerHandle`)))

(fn `UpdateAnimations`
  (params (AnimState :type "/Game/Core/Enums/E_AnimationStates Enum" :default "NewEnumerator0"))
  (switch `/Game/Core/Enums/E_AnimationStates` AnimState
    (:`NewEnumerator0`
      (set `self.CurrentAnimationState` "NewEnumerator0"))
    (:`NewEnumerator1`
      (set `self.CurrentAnimationState` "NewEnumerator1"))
    (:`NewEnumerator2`
      (set `self.CurrentAnimationState` "NewEnumerator2"))
    (:`NewEnumerator3`
      (set `self.CurrentAnimationState` "NewEnumerator2")))
  (`PaperFlipbookComponent.SetFlipbook` (`self.Sprite`) (select `/Game/Core/Enums/E_AnimationStates` (`self.CurrentAnimationState`) :`NewEnumerator0` (`self.IdleFlipbook`) :`NewEnumerator1` (`self.RunFlipbook`) :`NewEnumerator2` (`self.JumpingFlipbook`) :`NewEnumerator3` (`self.LandingFlipbook`))))

(fn `UserConstructionScript`
  (set `self.JumpMaxCount` (`self.JumpCount`))
  (set `self.JumpMaxHoldTime` (`self.MaxJumpHoldTime`))
  (set `CharacterMovementComponent.MaxWalkSpeed` (`self.DefaultMovementSpeed`) (`self.CharacterMovement`)))